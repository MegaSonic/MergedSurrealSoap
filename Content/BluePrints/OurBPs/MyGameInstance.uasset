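; Game instance that tracks the player's current quest, manages its dialogue and quest widgets, and sets the default commander pawn by faction.
; CreateNewQuest loads a fixed first entry from Dialogue data and shows the dialogue widget, while CreateANewQuest separately shows the quest widget.
; QuestDetect adds matching event counts toward the goal, then CompleteQuest restores default quest data and removes both widgets without resetting progress.
; CreateANewDialogue is an empty stub.
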(event `QuestDetect`
  (params (QuestEvent :type "/Game/QuestEnum Enum") (QuestCount :type Byte))
  (bind (_currentquest_questdescription _currentquest_questtext _currentquest_questtype _currentquest_questgoal) (break `/Game/OneQuest` (`self.CurrentQuest`)))
  (`KismetSystemLibrary.PrintString` (`|GetEnumeratorNameAsString` _currentquest_questtype))
  (if (`|EnumEquality` QuestEvent _currentquest_questtype)
    (bind _output_get (set `self.currentQuestProgress` (+ (`self.currentQuestProgress`) QuestCount)))
    (if (>= _output_get _currentquest_questgoal)
      (`self.CompleteQuest`))))

(event `CreateANewQuest`
  (bind _returnvalue (`|CreateWidget` "/Game/Widgets/Quest.Quest_C" (`GameplayStatics.GetPlayerController` 0)))
  (set `self.CurrentDisplayQuest` _returnvalue)
  (`UserWidget.AddToViewport` _returnvalue 0))

(event `CompleteQuest`
  (bind (_dialogue_text1 _dialogue_text2 _dialogue_text3 _dialogue_text4 _dialogue_quest_text1 _dialogue_quest_text2 _dialogue_quest_text3 _dialogue_quest_text4 _dialogue_quest1_request _dialogue_quest2_request _dialogue_quest3_request _dialogue_quest4_request _dialogue_quest1_count _dialogue_quest2_count _dialogue_quest3_count _dialogue_quest4_count _dialogue_textdefault _dialogue_quest_text_default _dialogue_quest_request_default _dialogue_quset_count_default) (break `/Game/Widgets/DialogueStruct` (`self.Dialogue`)))
  (`KismetSystemLibrary.PrintString` "Complete!!")
  (bind _output_get (set `self.CurrentQuest` (make `/Game/OneQuest` _dialogue_textdefault _dialogue_quest_text_default _dialogue_quest_request_default _dialogue_quset_count_default)))
  (`KismetSystemLibrary.PrintString` (`|GetEnumeratorNameAsString` (`.QuestType_7_53A938CF477B469E65977E95DCDFCE6E` (break `/Game/OneQuest` _output_get))))
  (`Widget.RemoveFromParent` (`self.CurrentDisplayQuest`))
  (`Widget.RemoveFromParent` (`self.CurrentDisplayDialogue`)))

(fn `ChooseOneDialogueAndQuest`
  (returns (QuestText :type Text) (QuestDescription :type Text) (QuestType :type "/Game/QuestEnum Enum") (QuestRequest :type Byte))
  (bind (_text1 _text2 _text3 _text4 _quest_text1 _quest_text2 _quest_text3 _quest_text4 _quest1_request _quest2_request _quest3_request _quest4_request _quest1_count) (break `/Game/Widgets/DialogueStruct` (`self.Dialogue`)))
  (return _text1 _quest_text1 _quest1_request _quest1_count))

(fn `CreateANewDialogue`)

(fn `CreateNewQuest`
  (bind (_questtext _questdescription _questtype _questrequest) (`self.ChooseOneDialogueAndQuest`))
  (set `self.CurrentQuest` (make `/Game/OneQuest` _questdescription _questtext _questtype _questrequest))
  (bind _returnvalue (`|CreateWidget` "/Game/Widgets/Dialogue.Dialogue_C" (`GameplayStatics.GetPlayerController` 0)))
  (`UserWidget.AddToViewport` _returnvalue 0)
  (set `self.CurrentDisplayDialogue` _returnvalue))

(fn `setDefaultPawn`
  (switch `name` (`self.FactionName`)
    (:`Humans`
      (set `self.DefaultPawn` "/Game/BluePrints/Units/Units/Commanders/HumanCommander.HumanCommander_C"))
    (:`Alliens`
      (set `self.DefaultPawn` "/Game/BluePrints/Units/Units/Commanders/AllienCommander.AllienCommander_C"))))