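; BP_Clock is an interactable clock actor with animated hour and minute hands.
; Tick advances a wrapping Time value scaled by Speed, and UpdateHands converts it to each hand's relative pitch using modulo cycles.
; On interaction, a character within range is marked Using, turned to face the clock, and one energy is deducted from the game instance's HUD.
; Characters out of range are sent toward the interaction location instead.
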(event `self.ReceiveTick`
  (params (DeltaSeconds :type "Float (single-precision)"))
  (set `self.Time` (mod (+ (/ (* DeltaSeconds (`self.Speed`)) 360.0) (`self.Time`)) (`self.TWO_PI`)))
  (`self.UpdateHands`))

(event `/Game/BluePrints/Units/BPInterface.Interact_With_Things`
  (params (Interaction_Location :type "Vector Structure") (ObjectType :type Integer) (TargetCharacter :type "/Game/BluePrints/Units/MyCharacter Object Reference"))
  (bind (_returnvalue_roll _returnvalue_pitch) (`KismetMathLibrary.BreakRotator` (`self.K2_GetActorRotation` TargetCharacter)))
  (bind (_returnvalue_roll_2 _returnvalue_pitch_2 _returnvalue_yaw) (`KismetMathLibrary.BreakRotator` (`KismetMathLibrary.Conv_VectorToRotator` (- (`self.K2_GetActorLocation` self) (`self.K2_GetActorLocation` TargetCharacter)))))
  (if (<= (`self.GetDistanceTo` self TargetCharacter) 200.0)
    (set `/Game/BluePrints/Units/MyCharacter.using?` true TargetCharacter)
    (`self.K2_SetActorRotation` TargetCharacter (`KismetMathLibrary.MakeRotator` _returnvalue_roll _returnvalue_pitch _returnvalue_yaw) false)
    (bind _asmy_game_instance (cast `/Game/BluePrints/OurBPs/MyGameInstance` (`GameplayStatics.GetGameInstance`)))
    (bind _gamehudenergy (`/Game/BluePrints/OurBPs/MyGameInstance.GameHudEnergy` _asmy_game_instance))
    (set `/Game/BluePrints/BP_Energy.currentEnergy` (- (`/Game/BluePrints/BP_Energy.currentEnergy` _gamehudenergy) 1) _gamehudenergy)
    (else
      (message `/Game/BluePrints/Units/BPInterface.Move_Character_To` TargetCharacter Interaction_Location))))

(fn `UpdateHands`
  (bind _two_pi_div_12 (`self.TWO_PI_DIV_12`))
  (bind _two_pi_div_60 (`self.TWO_PI_DIV_60`))
  ;[1 1 1] Hour Hand
  (`SceneComponent.K2_SetRelativeRotation` (`self.HourHand`) (`KismetMathLibrary.MakeRotator` 0.0 (* (/ (mod (`self.Time`) _two_pi_div_12) _two_pi_div_12) 360.0)) false false)
  ;[1 1 1] Minute Hand
  (`SceneComponent.K2_SetRelativeRotation` (`self.MinuteHand`) (`KismetMathLibrary.MakeRotator` 0.0 (* (/ (mod (`self.Time`) _two_pi_div_60) _two_pi_div_60) 360.0)) false false))

(fn `UserConstructionScript`)