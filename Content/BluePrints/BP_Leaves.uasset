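; BP_Leaves is an interactable leaves actor that a character can shake at a cost of energy.
; Within range, interaction flags the character as using, turns it to face the leaves, raises the particle emission rate through StartShake and deducts energy via the game instance's HUD.
; Out of range, it sends the character toward the interaction location instead.
; StartShake sets a Shaking flag but ignores its ShakeTime input, and nothing here resets the shake.
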(event `/Game/BluePrints/Units/BPInterface.Interact_With_Things`
  (params (Interaction_Location :type "Vector Structure") (ObjectType :type Integer) (TargetCharacter :type "/Game/BluePrints/Units/MyCharacter Object Reference"))
  (bind (_returnvalue_roll _returnvalue_pitch) (`KismetMathLibrary.BreakRotator` (`self.K2_GetActorRotation` TargetCharacter)))
  (bind (_returnvalue_roll_2 _returnvalue_pitch_2 _returnvalue_yaw) (`KismetMathLibrary.BreakRotator` (`KismetMathLibrary.Conv_VectorToRotator` (- (`self.K2_GetActorLocation` self) (`self.K2_GetActorLocation` TargetCharacter)))))
  (if (<= (`self.GetDistanceTo` self TargetCharacter) 500.0)
    (set `/Game/BluePrints/Units/MyCharacter.using?` true TargetCharacter)
    (`self.K2_SetActorRotation` TargetCharacter (`KismetMathLibrary.MakeRotator` _returnvalue_roll _returnvalue_pitch _returnvalue_yaw) false)
    (`self.StartShake` 200.0)
    (bind _asmy_game_instance (cast `/Game/BluePrints/OurBPs/MyGameInstance` (`GameplayStatics.GetGameInstance`)))
    (bind _gamehudenergy (`/Game/BluePrints/OurBPs/MyGameInstance.GameHudEnergy` _asmy_game_instance))
    (set `/Game/BluePrints/BP_Energy.currentEnergy` (- (`/Game/BluePrints/BP_Energy.currentEnergy` _gamehudenergy) 1) _gamehudenergy)
    (else
      (message `/Game/BluePrints/Units/BPInterface.Move_Character_To` TargetCharacter Interaction_Location))))

(fn `StartShake`
  (params (LeafCount :type "Float (double-precision)") (ShakeTime :type "Float (double-precision)"))
  (`ParticleSystemComponent.SetFloatParameter` (`self.ParticleSystem`) "EmissionRate" LeafCount)
  (set `self.Shaking` true))

(fn `UserConstructionScript`)