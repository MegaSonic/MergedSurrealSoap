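; BP_FloatingPiece is an actor that bobs up and down in the world.
; Its construction script randomizes the starting phase Theta, so separate instances can float out of sync.
; Each tick, DoFloat advances Theta by FloatSpeed times delta time, wrapped at two pi.
; It then adds a vertical offset of sin(Theta) times FloatHeight, unscaled by delta time, so travel depends on frame rate.
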(event `self.ReceiveTick`
  (params (DeltaSeconds :type "Float (single-precision)"))
  (`self.DoFloat` DeltaSeconds))

(fn `DoFloat`
  (params (`Delta Time` :type "Float (double-precision)"))
  (locals (TWOPI :type "Float (double-precision)" :default 6.283185))
  (bind _output_get (set `self.Theta` (mod (+ (* `Delta Time` (`self.FloatSpeed`)) (`self.Theta`)) (`local.TWOPI`))))
  (`self.K2_AddActorWorldOffset` (`KismetMathLibrary.MakeVector` 0.0 0.0 (* (`KismetMathLibrary.Sin` _output_get) (`self.FloatHeight`)))))

(fn `UserConstructionScript`
  (locals (TWOPI :type "Float (double-precision)" :default 6.283185))
  (set `self.Theta` (`KismetMathLibrary.RandomFloatInRange` 0.0 (`local.TWOPI`))))