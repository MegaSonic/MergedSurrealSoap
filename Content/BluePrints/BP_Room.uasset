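; BP_Room is a room actor that gains experience from the characters inside it and pays out currency when it ranks up.
; About once a second, Tick counts MyCharacter actors overlapping Cube1 and adds that number to the room's EXP.
; On reaching the threshold, it raises the rank, pays the BP_Currency actor found at BeginPlay, resets EXP, and doubles both threshold and next reward.
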(event `self.ReceiveBeginPlay`
  (bind _outactors (`GameplayStatics.GetAllActorsOfClass` "/Game/BluePrints/BP_Currency.BP_Currency_C"))
  (set `self.currency` (`KismetArrayLibrary.Array_Get` _outactors)))

(event `self.ReceiveTick`
  (params (DeltaSeconds :type "Float (single-precision)"))
  (bind _output_get (set `self.timer` (+ DeltaSeconds (`self.timer`))))
  (if (> _output_get 1.0)
    (bind _output_get_2 (set `self.actorsInRoom` (`KismetArrayLibrary.Array_Length` (`PrimitiveComponent.GetOverlappingActors` (`self.Cube1`) "/Game/BluePrints/Units/MyCharacter.MyCharacter_C"))))
    (set `self.roomEXP` (+ _output_get_2 (`self.roomEXP`)))
    (set `self.timer` 0.0)
    (if (>= (`self.roomEXP`) (`self.roomMaxEXP`))
      (set `self.roomRank` (+ (`self.roomRank`) 1))
      (bind _output_get_3 (set `/Game/BluePrints/BP_Currency.currentCurrency` (+ (stale _output_get_3) (`self.currencyOnRankUp`)) (`self.currency`)))
      (set `self.roomEXP` 0)
      (bind _output_get_4 (set `self.currencyOnRankUp` (* (stale _output_get_4) 2)))
      (bind _output_get_5 (set `self.roomMaxEXP` (* (stale _output_get_5) 2))))))

(fn `UserConstructionScript`)