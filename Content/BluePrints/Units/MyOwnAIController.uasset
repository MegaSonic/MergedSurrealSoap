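; AI controller for MyCharacter units, handling move orders, staged conversations and energy spending.
; Move orders use simple move-to-location and clear the pawn's Attacking flag.
; Talking sets Attacking on both characters, turns them to face each other by yaw, then prints hardcoded dialogue through staggered delays in a Sequence.
; A separate event decrements the current energy on the Game Instance's energy HUD.
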(event `/Game/BluePrints/Units/BPInterface.Move_Character_To`
  (params (location :type "Vector Structure"))
  (`NavigationSystem.SimpleMoveToLocation` self location)
  (bind _asmy_character (cast `/Game/BluePrints/Units/MyCharacter` (`self.K2_GetPawn` self)))
  (set `/Game/BluePrints/Units/MyCharacter.attacking?` false _asmy_character))

(event `/Game/BluePrints/Units/BPInterface.Talk_To_Character`
  (params (target :type "/Game/BluePrints/Units/MyCharacter Object Reference") (TalkLocation :type "Vector Structure"))
  (set `/Game/BluePrints/Units/MyCharacter.attacking?` true target)
  (bind _asmy_character (cast `/Game/BluePrints/Units/MyCharacter` (`self.K2_GetPawn` self)))
  (set `/Game/BluePrints/Units/MyCharacter.attacking?` true _asmy_character)
  (bind (_returnvalue_roll _returnvalue_pitch) (`KismetMathLibrary.BreakRotator` (`self.K2_GetActorRotation` _asmy_character)))
  (`self.K2_SetActorRotation` _asmy_character (`KismetMathLibrary.MakeRotator` _returnvalue_roll _returnvalue_pitch (.yaw (`KismetMathLibrary.Conv_VectorToRotator` (- TalkLocation (`self.K2_GetActorLocation` _asmy_character))))) false)
  (bind (_returnvalue_roll_2 _returnvalue_pitch_2 _returnvalue_yaw) (`KismetMathLibrary.BreakRotator` (`KismetMathLibrary.Conv_VectorToRotator` (- (`self.K2_GetActorLocation` _asmy_character) (`self.K2_GetActorLocation` target)))))
  (`self.K2_SetActorRotation` target (`KismetMathLibrary.MakeRotator` (.roll (`self.K2_GetActorRotation` target)) (.pitch (`self.K2_GetActorRotation` target)) _returnvalue_yaw) false)
  (`|ExecutionSequence`
    (:`then_0`
      (`KismetSystemLibrary.PrintString` "How's it going?"))
    (:`then_1`
      (`KismetSystemLibrary.Delay` 2.0)
      (`KismetSystemLibrary.PrintString` "Pretty good. You?" true true (struct :`G` 0.66 :`B` 1.0 :`A` 1.0) 6.0))
    (:`then_2`
      (`KismetSystemLibrary.Delay` 4.0)
      (`KismetSystemLibrary.PrintString` "Just so-so. Hey, did you hear that Arron get a 0 for his latest assignment?" true true (struct :`G` 0.66 :`B` 1.0 :`A` 1.0) 6.0))
    (:`then_3`
      (`KismetSystemLibrary.Delay` 6.0)
      (`KismetSystemLibrary.PrintString` "No way! He works hard I think!" true true (struct :`G` 0.66 :`B` 1.0 :`A` 1.0) 6.0))
    (:`then_4`
      (`KismetSystemLibrary.Delay` 8.0)
      (`KismetSystemLibrary.PrintString` "Yeah... But he kinda had a crush on a girl and now he's totally distracated...." true true (struct :`G` 0.66 :`B` 1.0 :`A` 1.0) 6.0))
    (:`then_5`
      (`KismetSystemLibrary.Delay` 10.0)
      (`KismetSystemLibrary.PrintString` "Alright Now you gotta tell me the name of that girl." true true (struct :`G` 0.66 :`B` 1.0 :`A` 1.0) 6.0))))

(event `/Game/BluePrints/HUDInterface.ConsumeEnergy`
  (params (AmountEnergy :type Integer))
  (bind _asmy_game_instance (cast `/Game/BluePrints/OurBPs/MyGameInstance` (`GameplayStatics.GetGameInstance`)))
  (bind _gamehudenergy (`/Game/BluePrints/OurBPs/MyGameInstance.GameHudEnergy` _asmy_game_instance))
  (set `/Game/BluePrints/BP_Energy.currentEnergy` (- (`/Game/BluePrints/BP_Energy.currentEnergy` _gamehudenergy) 1) _gamehudenergy))

(fn `UserConstructionScript`)