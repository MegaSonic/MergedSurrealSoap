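; Unit character Blueprint that carries out move and talk commands through MyOwnAIController and can become the player's camera view target.
; Talk requests start immediately within range, otherwise the unit walks toward the target and Tick starts the talk on arrival, stopping both characters.
; Tick also clears both characters' Attacking flags whenever they are out of range.
; A random happy mood is rolled on BeginPlay.
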(event `self.ReceiveBeginPlay`
  (if (< (`KismetMathLibrary.RandomIntegerInRange` 0 10) 6)
    (set `self.isHappy` true)
    (else
      (set `self.isHappy` false))))

(event `Look At Me`
  (bind _asmy_play_controller (cast `/Game/BluePrints/OurBPs/MyPlayController` (`GameplayStatics.GetPlayerController` 0)))
  (`PlayerController.SetViewTargetWithBlend` _asmy_play_controller self 1.0 "VTBlend_Linear" 0.0 false))

(event `/Game/BluePrints/Units/BPInterface.Move_Character_To`
  (params (location :type "Vector Structure"))
  (bind _asmy_own_aicontroller (cast `/Game/BluePrints/Units/MyOwnAIController` (`self.GetController`)))
  (`/Game/BluePrints/Units/MyOwnAIController.Move_Character_To` _asmy_own_aicontroller location)
  (set `self.using?` false)
  (set `self.attacking?` false))

(event `/Game/BluePrints/Units/BPInterface.Talk_To_Character`
  (params (target :type "/Game/BluePrints/Units/MyCharacter Object Reference") (TalkLocation :type "Vector Structure"))
  (bind _asmy_own_aicontroller (cast `/Game/BluePrints/Units/MyOwnAIController` (`self.GetController`)))
  (bind _output_get (set `self.InteractivePerson` target))
  (if (<= (`self.GetDistanceTo` _output_get self) 200.0)
    (`Controller.StopMovement` _asmy_own_aicontroller)
    (`/Game/BluePrints/Units/MyOwnAIController.Talk_To_Character` _asmy_own_aicontroller _output_get TalkLocation)
    (else
      (`/Game/BluePrints/Units/MyOwnAIController.Move_Character_To` _asmy_own_aicontroller (`self.K2_GetActorLocation` _output_get))
      (set `self.ApproahForATalk` true)))
  (message `/Game/BluePrints/HUDInterface.ConsumeEnergy` _asmy_own_aicontroller 1))

(event `self.ReceiveTick`
  (params (DeltaSeconds :type "Float (single-precision)"))
  (bind _interactiveperson (`self.InteractivePerson`))
  (if (!= _interactiveperson null)
    (if (<= (`self.GetDistanceTo` _interactiveperson self) 200.0)
      (if (`self.ApproahForATalk`)
        (`Controller.StopMovement` (`self.GetController` self))
        (`Controller.StopMovement` (`self.GetController` (`self.InteractivePerson`)))
        (bind _asmy_own_aicontroller (cast `/Game/BluePrints/Units/MyOwnAIController` (`self.GetController`)))
        (`/Game/BluePrints/Units/MyOwnAIController.Talk_To_Character` _asmy_own_aicontroller _interactiveperson (`self.K2_GetActorLocation` _interactiveperson))
        (set `self.ApproahForATalk` false))
      (else
        (set `self.attacking?` false)
        (set `/Game/BluePrints/Units/MyCharacter.attacking?` false (`self.InteractivePerson`))))))

(fn `ClearStates`
  (set `self.using?` false)
  (set `self.attacking?` false)
  (set `self.ApproahForATalk` false))

(fn `UserConstructionScript`)