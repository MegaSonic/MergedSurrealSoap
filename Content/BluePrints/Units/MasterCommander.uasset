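; Player commander pawn for mouse-driven character control, with basic touch selection and control of the level's "MyCamera" actor.
; Left click selects a MyCharacter and opens a gate so right click can move it, talk to another character or use a BP_Clock.
; B toggles buying mode, where short axis traces mount clocks on surfaces and report to GameInstance quests.
; Macros handle middle-mouse rotate, Shift pan and height-limited wheel zoom; H resets the view.
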(event `Key|Gesture_Flick`
  (params (Key :type "Key Structure" :default "AnyKey"))
  ;[1 1 1] Touch Controls
)

(event `InputTouch`
  (params (Location :type "Vector Structure") (FingerIndex :type "ETouchIndex Enum"))
  ;[1 1 1] Touch Controls
  (:`Pressed`
    (bind _asmy_character (cast `/Game/BluePrints/Units/MyCharacter` (`.HitActor` (`GameplayStatics.BreakHitResult` (`PlayerController.GetHitResultUnderFingerByChannel` (`GameplayStatics.GetPlayerController` 0) FingerIndex "TraceTypeQuery3" true))))
      (:`then`
        (`/Game/BluePrints/Units/MyCharacter.Look At Me` _asmy_character)
        (set `/Game/BluePrints/Units/MyCharacter.attacking?` false _asmy_character)
        (set `self.currentSelectActor` _asmy_character))
      (:`CastFailed`
        (set `self.currentSelectActor` null)
        (`self.Camera_Zoom` :!via `Zoom Out`)))))

(event `Key|Gesture_Pinch`
  (params (Key :type "Key Structure" :default "AnyKey"))
  ;[1 1 1] Touch Controls
)

(event `self.ReceiveBeginPlay`
  ;[1 1 1] Get The default main camera
  (set `PlayerController.bShowMouseCursor` true (`GameplayStatics.GetPlayerController` 0))
  (bind _outactors (`GameplayStatics.GetAllActorsOfClass` "/Script/Engine.CameraActor"))
  (for _array_element _outactors
    (if (`KismetStringLibrary.EqualEqual_StrStr` (`KismetSystemLibrary.GetDisplayName` _array_element) "MyCamera")
      (bind _output_get (set `self.TheSceneCamera` _array_element))
      (set `self.OriginCameraPosition` (`self.K2_GetActorLocation` _output_get))
      (bind _output_get_2 (set `self.TheSceneCamera` _array_element))
      (bind _output_get_3 (set `self.OriginCameraRotation` (`self.K2_GetActorRotation` _output_get_2)))
      (`KismetSystemLibrary.PrintString` (`KismetStringLibrary.Conv_RotatorToString` _output_get_3)))))

(event `InputAxis|MoveForward`
  (params (AxisValue :type "Float (single-precision)"))
  ;[1 1 1] Move the Pawn : not using now
  (`self.Camera_MoveForwardAndBack` AxisValue (stale `InputAxis|MoveRight` AxisValue) :!label _label))

(event `InputAxis|MoveRight`
  (params (AxisValue :type "Float (single-precision)"))
  ;[1 1 1] Move the Pawn : not using now
  (goto _label :!via `LeftAndRight`))

(event `Key|MouseScrollUp`
  (params (Key :type "Key Structure" :default "AnyKey"))
  ;[1 1 1] Mouse For Camera: Zoom in / Zoom out stuff.
  (:`Pressed`
    (`self.Camera_Zoom` :!label _label_2)))

(event `InputAxisKey|MouseX`
  (params (AxisValue :type "Float (single-precision)"))
  ;[1 1 1] Mouse For Camera: Zoom in / Zoom out stuff.
  (`/Engine/EditorBlueprintResources/StandardMacros.Gate` true :!label _label_3
    (:`Exit`
      (if (`self.Camera_TPanFRot`)
        (`self.Camera_Pan` AxisValue (stale `InputAxisKey|MouseY` AxisValue) :!label _label_4)
        (else
          (`self.Camera_Rotate` AxisValue (stale `InputAxisKey|MouseY` AxisValue) :!label _label_5))))))

(event `Key|MouseScrollDown`
  (params (Key :type "Key Structure" :default "AnyKey"))
  ;[1 1 1] Mouse For Camera: Zoom in / Zoom out stuff.
  (:`Pressed`
    (goto _label_2 :!via `Zoom Out`)))

(event `Key|MiddleMouseButton`
  (params (Key :type "Key Structure" :default "AnyKey"))
  ;[1 1 1] Mouse For Camera: Zoom in / Zoom out stuff.
  (:`Pressed`
    (set `self.Camera_CameraScreenEdgeHit` false)
    (`|ExecutionSequence`
      (:`then_0`
        (goto _label_3 :!via `Open`))
      (:`then_1`
        (goto _label_6 :!via `Open`))))
  (:`Released`
    (set `self.Camera_CameraScreenEdgeHit` true)
    (`|ExecutionSequence`
      (:`then_0`
        (goto _label_3 :!via `Close`))
      (:`then_1`
        (goto _label_6 :!via `Close`)))))

(event `InputAxisKey|MouseY`
  (params (AxisValue :type "Float (single-precision)"))
  ;[1 1 1] Mouse For Camera: Zoom in / Zoom out stuff.
  (`/Engine/EditorBlueprintResources/StandardMacros.Gate` true :!label _label_6
    (:`Exit`
      (if (`self.Camera_TPanFRot`)
        (goto _label_4 :!via `MouseY`)
        (else
          (goto _label_5 :!via `MouseY`))))))

(event `Key|LeftShift`
  (params (Key :type "Key Structure" :default "AnyKey"))
  ;[1 1 1] Mouse For Camera: Zoom in / Zoom out stuff.
  (:`Pressed`
    (set `self.Camera_TPanFRot` true))
  (:`Released`
    (set `self.Camera_TPanFRot` false)))

(event `Key|H`
  (params (Key :type "Key Structure" :default "AnyKey"))
  (bind _thescenecamera (`self.TheSceneCamera`))
  ;[1 1 1] H For reset the default Camera
  (:`Pressed`
    (`self.K2_SetActorLocation` _thescenecamera (`self.OriginCameraPosition`) false false)
    (`self.K2_SetActorRotation` _thescenecamera (`self.OriginCameraRotation`) false)
    (bind _asmy_play_controller (cast `/Game/BluePrints/OurBPs/MyPlayController` (`GameplayStatics.GetPlayerController` 0)))
    (`PlayerController.SetViewTargetWithBlend` _asmy_play_controller _thescenecamera 1.0 "VTBlend_Linear" 0.0 false)))

(event `Key|RightMouseButton`
  (params (Key :type "Key Structure" :default "AnyKey"))
  (bind (_bblockinghit _binitialoverlap _time _location _impactpoint _normal _impactnormal _physmat _hitactor) (`GameplayStatics.BreakHitResult` (`PlayerController.GetHitResultUnderCursorByChannel` (`GameplayStatics.GetPlayerController` 0) "TraceTypeQuery3" true)))
  ;[1 1 1] Left Click to select a character, and then right click to move it, if right click on another character, then interact with it..expanding now
  (:`Pressed`
    (`/Engine/EditorBlueprintResources/StandardMacros.Gate` true :!label _label_7
      (:`Exit`
        (bind _asmy_character (cast `/Game/BluePrints/Units/MyCharacter` _hitactor)
          (:`then`
            (if (!= _asmy_character (stale `Key|LeftMouseButton` _asmy_character))
              (message `/Game/BluePrints/Units/BPInterface.Talk_To_Character` (stale `Key|LeftMouseButton` _asmy_character) _asmy_character _location)))
          (:`CastFailed`
            (bind _asbp_clock (cast `/Game/BluePrints/BP_Clock` _hitactor)
              (:`then`
                (message `/Game/BluePrints/Units/BPInterface.Interact_With_Things` _asbp_clock _location 0 (stale `Key|LeftMouseButton` _asmy_character)))
              (:`CastFailed`
                (message `/Game/BluePrints/Units/BPInterface.Move_Character_To` (stale `Key|LeftMouseButton` _asmy_character) (`.Location` (`GameplayStatics.BreakHitResult` (`PlayerController.GetHitResultUnderCursorByChannel` (`GameplayStatics.GetPlayerController` 0) "TraceTypeQuery3" true))))))))))))

(event `Key|LeftMouseButton`
  (params (Key :type "Key Structure" :default "AnyKey"))
  (bind (_bblockinghit _binitialoverlap _time _location _impactpoint _normal _impactnormal _physmat _hitactor) (`GameplayStatics.BreakHitResult` (`PlayerController.GetHitResultUnderCursorByChannel` (`GameplayStatics.GetPlayerController` 0) "TraceTypeQuery3" true)))
  (:`Pressed`
    (if (`self.BuyingMode`)
      (bind (_outhit _returnvalue) (`KismetSystemLibrary.LineTraceSingle` :`Start` _location :`End` (+ _location (2.0 0.0 0.0)) :`TraceChannel` "TraceTypeQuery3" :`DrawDebugType` "ForDuration"))
      (bind (_bblockinghit_2 _binitialoverlap_2 _time_2 _location_2 _impactpoint_2 _normal_2 _impactnormal_2 _physmat_2 _hitactor_2) (`GameplayStatics.BreakHitResult` _outhit))
      (cast `/Game/BluePrints/Units/MyCharacter` _hitactor_2
        (:`CastFailed`
          (cast `/Game/BluePrints/BP_Clock` _hitactor_2
            (:`CastFailed`
              (if _returnvalue
                (bind _returnvalue_2 (`|SpawnActorFromClass` "/Game/BluePrints/BP_Clock.BP_Clock_C" (`KismetMathLibrary.Conv_VectorToTransform` _impactpoint_2) "AdjustIfPossibleButAlwaysSpawn" "OverrideRootScale"))
                (if (!= _returnvalue_2 null)
                  (`self.K2_SetActorRotation` _returnvalue_2 (struct :`Yaw` -90.0) false)
                  (`self.K2_SetActorLocation` _returnvalue_2 (- (`self.K2_GetActorLocation` _returnvalue_2) (3.0 0.0 0.0)) false false)
                  (bind _asmy_game_instance (cast `/Game/BluePrints/OurBPs/MyGameInstance` (`GameplayStatics.GetGameInstance`)))
                  (`/Game/BluePrints/OurBPs/MyGameInstance.QuestDetect` _asmy_game_instance "NewEnumerator0" 1))
                (else
                  (bind (_outhit_2 _returnvalue_3) (`KismetSystemLibrary.LineTraceSingle` _location (- _location (0.0 2.0 0.0)) "TraceTypeQuery3"))
                  (bind (_bblockinghit_3 _binitialoverlap_3 _time_3 _location_3 _impactpoint_3 _normal_3 _impactnormal_3 _physmat_3 _hitactor_3) (`GameplayStatics.BreakHitResult` _outhit_2))
                  (cast `/Game/BluePrints/Units/MyCharacter` _hitactor_3
                    (:`CastFailed`
                      (cast `/Game/BluePrints/BP_Clock` _hitactor_3
                        (:`CastFailed`
                          (if _returnvalue_3
                            (bind _returnvalue_4 (`|SpawnActorFromClass` "/Game/BluePrints/BP_Clock.BP_Clock_C" (`KismetMathLibrary.Conv_VectorToTransform` _impactpoint_3) "AdjustIfPossibleButAlwaysSpawn" "OverrideRootScale"))
                            (if (!= _returnvalue_4 null)
                              (`self.K2_SetActorRotation` _returnvalue_4 (struct :`Yaw` -180.0) false)
                              (`self.K2_SetActorLocation` _returnvalue_4 (+ (`self.K2_GetActorLocation` _returnvalue_4) (0.0 3.0 0.0)) false false)
                              (bind _asmy_game_instance_2 (cast `/Game/BluePrints/OurBPs/MyGameInstance` (`GameplayStatics.GetGameInstance`)))
                              (`/Game/BluePrints/OurBPs/MyGameInstance.QuestDetect` _asmy_game_instance_2 "NewEnumerator0" 1)))))))))))))
      (else
        ;[1 1 1] Left Click to select a character, and then right click to move it, if right click on another character, then interact with it..expanding now
        (bind _asmy_character (cast `/Game/BluePrints/Units/MyCharacter` _hitactor)
          (:`then`
            (`/Game/BluePrints/Units/MyCharacter.Look At Me` _asmy_character)
            (`/Game/BluePrints/Units/MyCharacter.ClearStates` _asmy_character)
            (`|ExecutionSequence`
              (:`then_0`
                (goto _label_7 :!via `Open`))))
          (:`CastFailed`
            (goto _label_7 :!via `Close`)))))))

(event `Key|B`
  (params (Key :type "Key Structure" :default "AnyKey"))
  (:`Pressed`
    (bind _output_get (set `self.BuyingMode` (not (`self.BuyingMode`))))
    (if _output_get
      (`KismetSystemLibrary.PrintString` "BuyingMode")
      (else
        (`KismetSystemLibrary.PrintString` "BuyingEnd")))))

(fn `UserConstructionScript`)